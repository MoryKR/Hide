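; BP_Player is the player actor Blueprint, providing a tagger HUD and a networked attack.
; On BeginPlay it creates WBP_TaggerHUD and adds it to the viewport if BP_PlayerState flags the player as tagger.
; Attack input while Idle sends a server request, which rechecks authority and Idle state before multicasting.
; The multicast sets State to Attack and plays the attack montage on the mesh at increased speed.
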(event `self.ReceiveBeginPlay`
  ; Tagger HUD
  (bind _asbp_player_state (cast `/Game/02_Program/Actor/BP/Player/BP_PlayerState` (`self.PlayerState`)))
  (if (`/Game/02_Program/Actor/BP/Player/BP_PlayerState.IsTagger` _asbp_player_state)
    (bind _returnvalue (`|CreateWidget` "/Game/03_UI/03_Widget/Game/WBP_TaggerHUD.WBP_TaggerHUD_C"))
    (`UserWidget.AddToViewport` _returnvalue 0)))

(event `ProcessAttackInput`
  ; Net
  (switch `/Game/02_Program/Actor/BP/EState` (`self.State`)
    (:`NewEnumerator0`
      (`self.Server_RequestAttack`))))

(event `Server_RequestAttack`
  ; Net
  (`/Engine/EditorBlueprintResources/ActorMacros.Switch Has Authority`
    (:`Authority`
      (switch `/Game/02_Program/Actor/BP/EState` (`self.State`)
        (:`NewEnumerator0`
          (`self.Multicast_ProcessAttack`))))))

(event `Multicast_ProcessAttack`
  ; Net
  (`|ExecutionSequence`
    (:`then_0`
      (set `self.State` "NewEnumerator1"))
    (:`then_1`
      (`|PlayMontage` (`self.Mesh`) "/Game/02_Program/Actor/Anim/AM_Attack.AM_Attack" 2.0))))

(fn `UserConstructionScript`
  (`parent.UserConstructionScript`))