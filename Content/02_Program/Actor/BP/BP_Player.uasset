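; BP_Player is the player Blueprint, handling a networked attack action.
; Attack input requests the server when State is Idle, and the server re-checks authority and Idle before multicasting.
; The multicast sets State to Attack and plays the AM_Attack montage on the mesh at increased speed.
; Nothing in this Blueprint returns State to Idle.
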(event `self.ReceiveBeginPlay`)

(event `ProcessAttackInput`
  ; Net
  (switch `/Game/02_Program/Actor/BP/EState` (`self.State`)
    (:`NewEnumerator0`
      (`self.Server_RequestAttack`))))

(event `Server_RequestAttack`
  ; Net
  (`/Engine/EditorBlueprintResources/ActorMacros.Switch Has Authority`
    (:`Authority`
      (switch `/Game/02_Program/Actor/BP/EState` (`self.State`)
        (:`NewEnumerator0`
          (`self.Multicast_ProcessAttack`))))))

(event `Multicast_ProcessAttack`
  ; Net
  (`|ExecutionSequence`
    (:`then_0`
      (set `self.State` "NewEnumerator1"))
    (:`then_1`
      (`|PlayMontage` (`self.Mesh`) "/Game/02_Program/Actor/Anim/AM_Attack.AM_Attack" 2.0))))

(fn `UserConstructionScript`
  (`parent.UserConstructionScript`))