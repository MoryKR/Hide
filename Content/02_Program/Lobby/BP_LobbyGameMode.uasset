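; Lobby game mode that manages players before a match and launches the selected level.
; PostLogin gives each player state an incrementing "User" nickname.
; SaveConfig maps the level choice to a map name, defaulting to WaterWheel, and stores player and bot limits.
; TryStartGame checks that every player is ready, copies both limits to the GameInstance, then runs a ServerTravel console command to the saved map.
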(event `self.K2_PostLogin`
  (params (NewPlayer :type "PlayerController Object Reference"))
  ; Set NickName
  (bind _asbp_lobby_player_state (cast `/Game/02_Program/Lobby/BP_LobbyPlayerState` (`Controller.PlayerState` NewPlayer)))
  (bind _result (`/Engine/EditorBlueprintResources/StandardMacros.IncrementInt` (`self.NicknameIndex`))
    (:`  `
      (set `/Game/02_Program/Lobby/BP_LobbyPlayerState.Nickname` (`|FormatText` "User{0}" _result) _asbp_lobby_player_state))))

(event `TryStartGame`
  ; Start Game
  (if (`self.EveryBodyReady`)
    (bind _asbp_game_instance (cast `/Game/02_Program/BP_GameInstance` (`GameplayStatics.GetGameInstance`)))
    (set `/Game/02_Program/BP_GameInstance.MaxPlayerCount` (`self.MaxPlayerCount`) _asbp_game_instance)
    (set `/Game/02_Program/BP_GameInstance.MaxBotCount` (`self.MaxBotCount`) _asbp_game_instance)
    (`KismetSystemLibrary.ExecuteConsoleCommand` (`KismetStringLibrary.Concat_StrStr` "ServerTravel" " " (`self.LevelName`)) null)))

(fn `EveryBodyReady`
  (returns (Ready :type Boolean))
  (for _array_element (`GameStateBase.PlayerArray` (`GameplayStatics.GetGameState`))
    (bind _asbp_lobby_player_state (cast `/Game/02_Program/Lobby/BP_LobbyPlayerState` _array_element))
    (if (not (`/Game/02_Program/Lobby/BP_LobbyPlayerState.Ready` _asbp_lobby_player_state))
      (return false)))
  (return true))

(fn `SaveConfig`
  (params (LevelName :type String) (InMaxPlayerCount :type Integer) (InMaxBotCount :type Integer))
  ; SaveConfig
  (`|ExecutionSequence`
    (:`then_0`
      (switch `string` (`self.LevelName`)
        (:`Default`
          (set `self.LevelName` "Level_WaterWheel" :!label _label))
        (:`Fountain`
          (set `self.LevelName` "Level_Fountain"))
        (:`Watermill`
          (goto _label))))
    (:`then_1`
      (set `self.MaxPlayerCount` InMaxPlayerCount)
      (set `self.MaxBotCount` InMaxBotCount))))

(fn `UserConstructionScript`)