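; Lobby player controller that relays a player's ready-button press and nickname change to the server.
; Each handler forwards to a server event, which reaches the lobby player state through the controlled pawn.
; Readying calls a multicast on that state, then asks the lobby game mode to try starting the game.
; Renaming writes the new nickname directly to the player state.
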(event `HandleReadyButton`
  ; Ready Button
  (`self.Server_HandleReadyButton`))

(event `Server_HandleReadyButton`
  ; Ready Button
  (if (`KismetSystemLibrary.IsServer`)
    (bind _asbp_lobby_player_state (cast `/Game/02_Program/Lobby/BP_LobbyPlayerState` (`Pawn.PlayerState` (`self.K2_GetPawn`))))
    (`/Game/02_Program/Lobby/BP_LobbyPlayerState.MultiCast_Ready` _asbp_lobby_player_state)
    (bind _asbp_lobby_game_mode (cast `/Game/02_Program/Lobby/BP_LobbyGameMode` (`GameplayStatics.GetGameMode`)))
    (`/Game/02_Program/Lobby/BP_LobbyGameMode.TryStartGame` _asbp_lobby_game_mode)))

(event `HandleChangeNickname`
  (params (`In NickName` :type Text))
  ; Change Nickname
  (`self.Server_HandleChangeNickname` `In NickName`))

(event `Server_HandleChangeNickname`
  (params (InNickName :type Text))
  ; Change Nickname
  (if (`KismetSystemLibrary.IsServer`)
    (bind _asbp_lobby_player_state (cast `/Game/02_Program/Lobby/BP_LobbyPlayerState` (`Pawn.PlayerState` (`self.K2_GetPawn`))))
    (set `/Game/02_Program/Lobby/BP_LobbyPlayerState.Nickname` InNickName _asbp_lobby_player_state)))

(fn `UserConstructionScript`)