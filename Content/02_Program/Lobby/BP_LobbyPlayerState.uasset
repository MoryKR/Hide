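; Lobby player state that holds a player's ready flag and nickname and keeps the lobby UI in sync with them.
; A multicast event sets Ready, and a RepNotify handles Nickname changes.
; Both, along with BeginPlay and destruction, refresh BP_LobbyHUD through the player controller.
; A client kick event sends a player removed by the server to the title level.
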(event `Client_Kicked`
  ; Kicked By Server
  (`GameplayStatics.OpenLevelBySoftObjectPtr` "/Game/00_Level/Level_Title.Level_Title"))

(event `MultiCast_Ready`
  (set `self.Ready` true)
  (`self.Refresh Lobby UI`))

(event `self.ReceiveBeginPlay`
  (`self.Refresh Lobby UI`)
  (add `self.OnDestroyed` (delegate `OnDestroyed_Event`)))

(event `OnDestroyed_Event` :!signature `self.OnDestroyed`
  (params (DestroyedActor :type "Actor Object Reference"))
  (`self.Refresh Lobby UI`))

(fn `OnRep_Nickname`
  (`self.Refresh Lobby UI`))

(fn `Refresh Lobby UI`
  (bind _returnvalue (`self.GetPlayerController`))
  (`/Engine/EditorBlueprintResources/StandardMacros.IsValid` _returnvalue
    (:`Is Valid`
      (bind _asbp_lobby_hud (cast `/Game/02_Program/Lobby/BP_LobbyHUD` (`PlayerController.GetHUD` _returnvalue)))
      (`/Game/02_Program/Lobby/BP_LobbyHUD.RefreshUI` _asbp_lobby_hud))))

(fn `UserConstructionScript`)